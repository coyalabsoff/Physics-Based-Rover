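; BP_Star_Generator builds a field of star sprites when play begins.
; GenerateStars clears its child components, then loops over rows and columns, adding a collision-free Paper sprite per cell with the configured sprite and color.
; Random multipliers on each grid coordinate scatter the stars across the XZ plane.
; X and Z scales are rolled separately, usually staying at a base size with an occasional random variation.
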(event EventBeginPlay
  (CallFunction|GenerateStars))

(fn ConstructionScript)

(fn GenerateStars
  (bind _returnvalue (|CalculateRandomStarSize))
  (CallFunction|ClearStars) ; Clear previous stars
  (for _index (range 0 (- (Variables|Default|GetRows) 1))
    (for _index_2 (range 0 (- (Variables|Default|GetColumns) 1))
      (bind _returnvalue_2 (AddComponent|AddPaperSpriteComponent false (Transformation|GetActorTransform)))
      (|SetSpriteProperties _returnvalue_2)
      (Transformation|SetRelativeLocation _returnvalue_2 (Math|Vector|MakeVector (|CalculateStarRow _index) 0.0 (|CalculateStarColumn _index_2)) false false)
      (Transformation|SetWorldScale3D _returnvalue_2 (Math|Vector|MakeVector _returnvalue 1.0 _returnvalue)))))

(fn ClearStars
  (for _index (range 0 15) ; Nothing to see here
    (Components|DestroyComponent (Components|GetChildrenComponents (Variables|Default|GetDefaultSceneRoot) true)))
  (Utilities|Platform|CollectGarbage))